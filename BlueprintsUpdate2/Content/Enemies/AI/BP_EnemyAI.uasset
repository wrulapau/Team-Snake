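; Enemy guard character that patrols waypoints, chases the player on sight and triggers a game over on contact.
; GuardPatrol walks to each waypoint in a looping array, pausing between stops.
; PawnSensing starts a faster chase, and a retriggerable delay returns it to patrol shortly after sightings stop.
; A capsule hit with the player shows the lose screen and pauses the game.
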(event `GuardPatrol`
  ; Patrol
  (set `CharacterMovementComponent.MaxWalkSpeed` 200.0 (`self.CharacterMovement`))
  (`|AIMoveTo` self (0.0 0.0 0.0) (`|GetArrayItem` (`self.Waypoints`) (`self.CurrentWaypoint`)) 10.0
    (:`OnSuccess`
      (`KismetSystemLibrary.PrintString` (`KismetStringLibrary.Conv_IntToString` (`self.CurrentWaypoint`)))
      (`/Engine/EditorBlueprintResources/StandardMacros.IncrementInt` (`self.CurrentWaypoint`)
        (:`  `
          (if (>= (`self.CurrentWaypoint`) (`KismetArrayLibrary.Array_Length` (`self.Waypoints`)))
            (set `self.CurrentWaypoint` 0))
          (`KismetSystemLibrary.Delay` 5.0)
          (`self.GuardPatrol`))))))

(event `self.ReceiveBeginPlay`
  ; If no player has been spotted, then keep patrolling
  (if (not (`self.CanSeePlayer?`))
    (`self.GuardPatrol`)))

(event `self.PawnSensing.OnSeePawn`
  (params (Pawn :type "Pawn Object Reference"))
  ; Chase Player
  (bind _asbp_third_person_character (cast `/Game/ThirdPerson/Blueprints/BP_ThirdPersonCharacter` Pawn))
  (`|ExecutionSequence`
    (:`then_0`
      (set `self.CanSeePlayer?` true)
      (set `CharacterMovementComponent.MaxWalkSpeed` 300.0 (`self.CharacterMovement`))
      (`|AIMoveTo` self (0.0 0.0 0.0) _asbp_third_person_character))
    (:`then_1`
      (`KismetSystemLibrary.RetriggerableDelay` 1.0)
      (set `self.CanSeePlayer?` false)
      (`self.GuardPatrol`))))

(event `self.CapsuleComponent.OnComponentHit`
  (params (HitComponent :type "PrimitiveComponent Object Reference") (OtherActor :type "Actor Object Reference") (OtherComp :type "PrimitiveComponent Object Reference") (NormalImpulse :type "Vector Structure") (Hit :type "HitResult Structure (by ref)"))
  (cast `/Game/ThirdPerson/Blueprints/BP_ThirdPersonCharacter` OtherActor)
  (`WidgetLayoutLibrary.RemoveAllWidgets`)
  (bind _returnvalue (`|CreateWidget` "/Game/_Main/Widget/W_LoseScreen.W_LoseScreen_C"))
  (`UserWidget.AddToViewport` _returnvalue 0)
  (`GameplayStatics.SetGamePaused` true))

(fn `UserConstructionScript`)