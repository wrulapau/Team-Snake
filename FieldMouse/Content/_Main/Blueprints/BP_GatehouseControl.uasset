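; Gatehouse control that lets a third-person character holding key item 1 operate a moving Cube, likely the gate.
; Box overlap scans the character's InventoryArray for that key and sets CanUseKey, which is cleared when the character leaves.
; ActivateKey prints a debug message and, for key 1, plays a Timeline that updates the Cube's relative location while preserving X and Y.
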(event `self.Box.OnComponentBeginOverlap`
  (params (OverlappedComponent :type "PrimitiveComponent Object Reference") (OtherActor :type "Actor Object Reference") (OtherComp :type "PrimitiveComponent Object Reference") (OtherBodyIndex :type Integer) (bFromSweep :type Boolean) (SweepResult :type "HitResult Structure (by ref)"))
  (bind _asbp_third_person_character (cast `/Game/ThirdPerson/Blueprints/BP_ThirdPersonCharacter` OtherActor))
  (for _array_element (`/Game/ThirdPerson/Blueprints/BP_ThirdPersonCharacter.InventoryArray` _asbp_third_person_character)
    (if (== (`.ItemKeyID_24_40F0A0174AF170EDE964DC84E7365589` (break `/Game/_Main/Structures/S_ItemStructure` _array_element)) 1)
      (set `/Game/ThirdPerson/Blueprints/BP_ThirdPersonCharacter.CanUseKey?` true _asbp_third_person_character))))

(event `self.Box.OnComponentEndOverlap`
  (params (OverlappedComponent :type "PrimitiveComponent Object Reference") (OtherActor :type "Actor Object Reference") (OtherComp :type "PrimitiveComponent Object Reference") (OtherBodyIndex :type Integer))
  (bind _asbp_third_person_character (cast `/Game/ThirdPerson/Blueprints/BP_ThirdPersonCharacter` OtherActor))
  (set `/Game/ThirdPerson/Blueprints/BP_ThirdPersonCharacter.CanUseKey?` false _asbp_third_person_character))

(event `/Game/_Main/Blueprints/BI_KeyInterface.ActivateKey`
  (params (ItemKeyID :type Integer))
  (bind _cube (`self.Cube`))
  (bind (_relativelocation_x _relativelocation_y) (`KismetMathLibrary.BreakVector` (`SceneComponent.RelativeLocation` _cube)))
  (`KismetSystemLibrary.PrintString` "KeyActivated")
  (if (== ItemKeyID 1)
    (`Timeline|Timeline`
      (:`Update`
        (`SceneComponent.K2_SetRelativeLocation` _cube (`KismetMathLibrary.MakeVector` _relativelocation_x _relativelocation_y) false false)))))

(fn `UserConstructionScript`)